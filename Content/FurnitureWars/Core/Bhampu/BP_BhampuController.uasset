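; BP_BhampuController is the player controller that links its C++ parent's stealth and dash logic to the HUD and the BP_Jonna pawn.
; Stealth volume events store the trigger, set the overlap flag and toggle the HUD prompt, while Tick refreshes the interaction prompt.
; Hide and unhide calls from C++ pass to the pawn with the volume, and StealthWarping stays set until Warped clears it.
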(event `self.ReceiveTick`
  (params (DeltaSeconds :type "Float (single-precision)"))
  (bind _mainhud (message `/Game/FurnitureWars/Core/Interfaces/BPI_GameMode.GetPlayerHUD` (`GameplayStatics.GetGameMode`)))
  (message `/Game/FurnitureWars/Core/Interfaces/BPI_MainHUD.PromptInteraction` _mainhud (`self.bInteractionAvailable`)))

(event `/Game/FurnitureWars/Core/Interfaces/BPI_StealthSystem.StealthVolumeEntered`
  (params (StealthTriggerRef :type "Actor Object Reference"))
  ;[1 1 1] Stealth System
  ;;[1 1 1] Stealth Volume Entered. Tell Cpp to accept stealth input and update HUD.
  (set `self.Stealth Trigger Ref` StealthTriggerRef)
  (bind _mainhud (message `/Game/FurnitureWars/Core/Interfaces/BPI_GameMode.GetPlayerHUD` (`GameplayStatics.GetGameMode`)))
  (message `/Game/FurnitureWars/Core/Interfaces/BPI_MainHUD.PromptStealth` _mainhud)
  (set `self.bStealthOverlap` true))

(event `self.ReceiveBeginPlay`
  ;[1 1 1] Begin Play
  (bind _mainhud (message `/Game/FurnitureWars/Core/Interfaces/BPI_GameMode.GetPlayerHUD` (`GameplayStatics.GetGameMode`)))
  (set `self.Main HUD` _mainhud))

(event `self.UIDashUpdate`
  (params (AbilityCooldownFraction :type "Float (single-precision)"))
  ;[1 1 1] DashUI
  (bind _mainhud (message `/Game/FurnitureWars/Core/Interfaces/BPI_GameMode.GetPlayerHUD` (`GameplayStatics.GetGameMode`)))
  (message `/Game/FurnitureWars/Core/Interfaces/BPI_MainHUD.SetDashCooldown` _mainhud AbilityCooldownFraction))

(event `/Game/FurnitureWars/Core/Interfaces/BPI_StealthSystem.StealthVolumeExited`
  ;[1 1 1] Stealth System
  ;;[1 1 1] Stealth Volume Exit. Tell Cpp to stop accepting stealth input and update HUD.
  (set `self.bStealthOverlap` false)
  (bind _mainhud (message `/Game/FurnitureWars/Core/Interfaces/BPI_GameMode.GetPlayerHUD` (`GameplayStatics.GetGameMode`)))
  (message `/Game/FurnitureWars/Core/Interfaces/BPI_MainHUD.RemoveStealth` _mainhud))

(event `self.PromptInteractionUI`
  (params (bInteraction :type Boolean))
  ;[1 1 1] Interaction UI
)

(event `self.ReadyToHide`
  ;[1 1 1] Stealth System
  ;;[1 1 1] Ready to Hide called from Cpp. Pass the message to BP_Jonna
  (set `self.bStealthWarping` true)
  (message `/Game/FurnitureWars/Core/Interfaces/BPI_StealthSystem.Hide` (`GameplayStatics.GetPlayerPawn` 0) true (`self.Stealth Trigger Ref`)))

(event `self.UnHide`
  ;[1 1 1] Stealth System
  ;;[1 1 1] UnHide called from Cpp. Pass it on to BP_Jonna
  (`parent.UnHide`)
  (message `/Game/FurnitureWars/Core/Interfaces/BPI_StealthSystem.Hide` (`GameplayStatics.GetPlayerPawn` 0) false (`self.Stealth Trigger Ref`)))

(event `/Game/FurnitureWars/Core/Interfaces/BPI_StealthSystem.Warped`
  ;[1 1 1] Stealth System
  ;;[1 1 1] BP_Jonna has finished stealth warp movement. Allow Cpp to accept movement input.
  (set `self.bStealthWarping` false))

(fn `GetCurrentStealthState`
  (returns (CurrentStealthState :type "/Game/FurnitureWars/Core/Systems/Stealth/E_StealthStates Enum"))
  (return "NewEnumerator0"))

(fn `GetWarpLocation`
  (returns (WarpLocation :type "Vector Structure"))
  (return (0.0 0.0 0.0)))

(fn `UserConstructionScript`)