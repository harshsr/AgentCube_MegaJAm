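; Game mode for Furniture Wars that manages the HUD, pause and quit flow, level progression and win or lose screens.
; It creates the main HUD on BeginPlay and exposes it through GetPlayerHUD.
; Events toggle pause, cursor and input mode, spawning pause, success or failure menus, the latter showing a fail reason.
; Restart and next-level events switch on the player pawn's current level to open the matching map.
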(event `self.ReceiveBeginPlay`
  (bind _returnvalue (`GameplayStatics.GetPlayerController` 0))
  (`WidgetBlueprintLibrary.SetInputMode_GameOnly` _returnvalue)
  (set `PlayerController.bShowMouseCursor` false _returnvalue)
  (bind _returnvalue_2 (`|CreateWidget` "/Game/FurnitureWars/Core/UI/HUD/WBP_MainHUD.WBP_MainHUD_C" (`GameplayStatics.GetPlayerController` 0)))
  (bind _output_get (set `self.HUD` _returnvalue_2))
  (`UserWidget.AddToViewport` _output_get 0))

(event `/Game/FurnitureWars/Core/Interfaces/BPI_GameMode.QuitGame`
  (`KismetSystemLibrary.QuitGame` null "Quit"))

(event `/Game/FurnitureWars/Core/Interfaces/BPI_GameMode.ResumeGame`
  (bind _returnvalue (`GameplayStatics.GetPlayerController` 0))
  (`WidgetBlueprintLibrary.SetInputMode_GameOnly` _returnvalue)
  (set `PlayerController.bShowMouseCursor` false _returnvalue)
  (`GameplayStatics.SetGamePaused` false))

(event `/Game/FurnitureWars/Core/Interfaces/BPI_GameMode.PauseGame`
  (bind _returnvalue (`GameplayStatics.GetPlayerController` 0))
  (`WidgetBlueprintLibrary.SetInputMode_UIOnlyEx` _returnvalue null)
  (set `PlayerController.bShowMouseCursor` true _returnvalue)
  (`GameplayStatics.SetGamePaused` true)
  (bind _returnvalue_2 (`|CreateWidget` "/Game/FurnitureWars/Core/UI/WBP_PauseMenu.WBP_PauseMenu_C"))
  (`UserWidget.AddToViewport` _returnvalue_2 0))

(event `/Game/FurnitureWars/Core/Interfaces/BPI_GameMode.RestartGame`
  (bind _returnvalue (`GameplayStatics.GetPlayerController` 0))
  (set `PlayerController.bShowMouseCursor` false _returnvalue)
  (`WidgetBlueprintLibrary.SetInputMode_GameOnly` _returnvalue)
  (bind _currentlevel (message `/Game/FurnitureWars/Core/Interfaces/BPI_Bhampu.GetCurrentLevel` (`GameplayStatics.GetPlayerPawn` 0)))
  (switch `/Game/FurnitureWars/Core/Systems/LevelSys/E_LevelNames` _currentlevel
    (:`NewEnumerator0`
      (`GameplayStatics.OpenLevelBySoftObjectPtr` "/Game/FurnitureWars/Maps/MainMenu.MainMenu"))
    (:`NewEnumerator1`
      (`GameplayStatics.OpenLevelBySoftObjectPtr` "/Game/FurnitureWars/Maps/Tutorial.Tutorial"))
    (:`NewEnumerator2`
      (`GameplayStatics.OpenLevelBySoftObjectPtr` "/Game/FurnitureWars/Maps/Latur.Latur"))
    (:`NewEnumerator3`
      (`GameplayStatics.OpenLevelBySoftObjectPtr` "/Game/FurnitureWars/Maps/Renapur.Renapur"))))

(event `/Game/FurnitureWars/Core/Interfaces/BPI_GameMode.NexLevel`
  (bind _returnvalue (`GameplayStatics.GetPlayerController` 0))
  (set `PlayerController.bShowMouseCursor` false _returnvalue)
  (`WidgetBlueprintLibrary.SetInputMode_GameOnly` _returnvalue)
  (bind _currentlevel (message `/Game/FurnitureWars/Core/Interfaces/BPI_Bhampu.GetCurrentLevel` (`GameplayStatics.GetPlayerPawn` 0)))
  (switch `/Game/FurnitureWars/Core/Systems/LevelSys/E_LevelNames` _currentlevel
    (:`NewEnumerator0`
      (`GameplayStatics.OpenLevelBySoftObjectPtr` "/Game/FurnitureWars/Maps/Tutorial.Tutorial"))
    (:`NewEnumerator1`
      (`GameplayStatics.OpenLevelBySoftObjectPtr` "/Game/FurnitureWars/Maps/Latur.Latur"))
    (:`NewEnumerator2`
      (`GameplayStatics.OpenLevelBySoftObjectPtr` "/Game/FurnitureWars/Maps/Renapur.Renapur"))
    (:`NewEnumerator3`
      (`GameplayStatics.OpenLevelBySoftObjectPtr` "/Game/FurnitureWars/Maps/MainMenu.MainMenu"))))

(event `/Game/FurnitureWars/Core/Interfaces/BPI_Tutorial.SuccessInLevel`
  (params (Success :type Boolean) (FailReason :type "/Game/FurnitureWars/Core/UI/FailureMenues/E_FailReason Enum" :default "NewEnumerator0"))
  (bind _returnvalue (`GameplayStatics.GetPlayerController` 0))
  (`GameplayStatics.SetGamePaused` true)
  (if Success
    (`WidgetBlueprintLibrary.SetInputMode_UIOnlyEx` _returnvalue null)
    (set `PlayerController.bShowMouseCursor` true _returnvalue)
    (bind _returnvalue_2 (`|CreateWidget` "/Game/FurnitureWars/Core/UI/FailureMenues/WBP_SuccessMenu.WBP_SuccessMenu_C" _returnvalue))
    (`UserWidget.AddToViewport` _returnvalue_2 0)
    (else
      (`WidgetBlueprintLibrary.SetInputMode_UIOnlyEx` _returnvalue null)
      (set `PlayerController.bShowMouseCursor` true _returnvalue)
      (bind _returnvalue_3 (`|CreateWidget` "/Game/FurnitureWars/Core/UI/FailureMenues/WBP_FailureMenu.WBP_FailureMenu_C" _returnvalue))
      (`UserWidget.AddToViewport` _returnvalue_3 0)
      (message `/Game/FurnitureWars/Core/Interfaces/BPI_Furniture.FailReason` _returnvalue_3 FailReason))))

(fn `GetPlayerHUD`
  (returns (MainHUD :type "Widget Object Reference"))
  (return (`self.HUD`)))

(fn `UserConstructionScript`)