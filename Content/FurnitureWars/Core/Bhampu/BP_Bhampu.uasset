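; Bhampu player pawn for Furniture Wars, with a gun that grabs and resizes furniture and the ability to hide in stealth volumes.
; Tick sphere-traces for BPI_Furniture actors, carries the held one by PhysicsHandle and updates HUD.
; Scaling is clamped per object; growing fills a shared energy meter, shrinking drains it.
; Hiding alerts all neighbour AI, timeline-warps Bhampu into the volume, swaps material and adds a stealth gameplay tag.
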(event `self.ReceiveBeginPlay`
  (`BlueprintGameplayTagLibrary.AddGameplayTag` (`self.BhampuTags`) (struct :`TagName` "Area.Neutral")))

(event `/Game/FurnitureWars/Core/Interfaces/BPI_Bhampu.AddTagToBhampuTags`
  (params (TagToAdd :type "GameplayTag Structure"))
  (`BlueprintGameplayTagLibrary.AddGameplayTag` (`self.BhampuTags`) TagToAdd))

(event `/Game/FurnitureWars/Core/Interfaces/BPI_Bhampu.RemoveTagFromBhampuTags`
  (params (TagToRemove :type "GameplayTag Structure"))
  (`BlueprintGameplayTagLibrary.RemoveGameplayTag` (`self.BhampuTags`) TagToRemove))

(event `/Game/FurnitureWars/Core/Interfaces/BPI_StealthSystem.ModifyCurrentStealthState`
  (params (CurrentStealthState :type "/Game/FurnitureWars/Core/Systems/Stealth/E_StealthStates Enum" :default "NewEnumerator0"))
  (set `self.CurrentStealthState` CurrentStealthState))

(event `/Game/FurnitureWars/Core/Interfaces/BPI_StealthSystem.Hide`
  (params (bHiding :type Boolean) (StealthVolumeRef :type "Actor Object Reference"))
  ;[1 1 1] Stealth Warp and meterial change when controller tells to hide
  (if bHiding
    ;;[1 1 1] Fix This. Might be too expensive
    (bind _outactors (`GameplayStatics.GetAllActorsOfClass` "/Game/FurnitureWars/AI/Neighbour/BP_Neighbour_AI.BP_Neighbour_AI_C")) ; Too Expensive
    (for _array_element _outactors
      (message `/Game/FurnitureWars/AI/Neighbour/BPI_Neighbour.CheckSpottedHiding` _array_element))
    (`BlueprintGameplayTagLibrary.AddGameplayTag` (`self.BhampuTags`) (struct :`TagName` "State.Stealth"))
    (bind (_direction _timealpha) (`Timeline|StealthWarpTimeline` :!via `PlayFromStart`)
      (:`Update`
        (bind _warplocation (message `/Game/FurnitureWars/Core/Interfaces/BPI_StealthSystem.GetWarpLocation` StealthVolumeRef))
        (`self.K2_SetActorLocation` (`KismetMathLibrary.VLerp` (`self.K2_GetActorLocation`) _warplocation _timealpha))
        (`PrimitiveComponent.SetMaterial` (`self.BaseSkelMesh`) 0 (`self.HiddenMat`)))
      (:`Finished`
        (`PrimitiveComponent.SetPhysicsLinearVelocity` (`self.BaseCollision`) (0.0 0.0 0.0) false "None")
        (`KismetSystemLibrary.Delay` 0.5)
        (`PrimitiveComponent.SetPhysicsLinearVelocity` (`self.BaseCollision`) (0.0 0.0 0.0) false "None")
        (message `/Game/FurnitureWars/Core/Interfaces/BPI_StealthSystem.Warped` (`GameplayStatics.GetPlayerController` 0))
        (`self.Hidden`)))
    (else
      (`PrimitiveComponent.SetMaterial` (`self.BaseSkelMesh`) 0 (`self.NormanlMat`)))))

(event `BhampuCppInterface.JumpAnim`
  (`SkeletalMeshComponent.PlayAnimation` (`self.BaseSkelMesh`) (`self.JumpAnimation`) false))

(event `/Game/FurnitureWars/Core/Interfaces/BPI_Bhampu.SetCurrentLevel`
  (params (CurrentLevel :type "/Game/FurnitureWars/Core/Systems/LevelSys/E_LevelNames Enum" :default "NewEnumerator0"))
  (set `self.CurrentLevel` CurrentLevel))

(event `self.BaseCollision.OnComponentHit`
  (params (HitComponent :type "PrimitiveComponent Object Reference") (OtherActor :type "Actor Object Reference") (OtherComp :type "PrimitiveComponent Object Reference") (NormalImpulse :type "Vector Structure") (Hit :type "HitResult Structure (by ref)"))
  ;[1 1 1] Jump reset on ground hit
  (if (`self.ActorHasTag` OtherActor "Ground")
    (set `self.bJumped` false)))

(event `InputAction|ScaleUp`
  (params (Key :type "Key Structure"))
  (:`Pressed`
    (if (`self.bCurrentlyHolding`)
      (`/Engine/EditorBlueprintResources/StandardMacros.IsValid` (`self.CurrentHeldActor`)
        (:`Is Valid`
          (set `self.bCanScaleUp` true))
        (:`Is Not Valid`
          (set `self.bCanScaleUp` false)))
      (else
        (set `self.bCanScaleUp` false))))
  (:`Released`
    (set `self.bCanScaleUp` false)))

(event `InputAction|ScaleDown`
  (params (Key :type "Key Structure"))
  (:`Pressed`
    (if (`self.bCurrentlyHolding`)
      (`/Engine/EditorBlueprintResources/StandardMacros.IsValid` (`self.CurrentHeldActor`)
        (:`Is Valid`
          (set `self.bCanScaleDown` true))
        (:`Is Not Valid`
          (set `self.bCanScaleDown` false)))
      (else
        (set `self.bCanScaleDown` false))))
  (:`Released`
    (set `self.bCanScaleDown` false)))

(event `InputAction|PauseMenu`
  (params (Key :type "Key Structure"))
  (:`Pressed`
    (message `/Game/FurnitureWars/Core/Interfaces/BPI_GameMode.PauseGame` (`GameplayStatics.GetGameMode`))))

(event `InputAction|Grab`
  (params (Key :type "Key Structure"))
  (:`Pressed`
    (if (`self.bGrabbableObjectFound`)
      (if (`self.bCurrentlyHolding`)
        (`self.ReleaseObject` :!label _label)
        (else
          (`self.GrabObject`)))
      (else
        (goto _label)))))

(event `self.ReceiveTick`
  (params (DeltaSeconds :type "Float (single-precision)"))
  (bind _returnvalue (`GameplayStatics.GetGameMode`))
  (bind _s_gun (`self.S_Gun`))
  (bind _s_gun_2 (`self.S_Gun`))
  (bind _returnvalue_2 (`SceneComponent.K2_GetComponentLocation` _s_gun_2))
  (set `self.Delta Seconds` DeltaSeconds)
  (`|ExecutionSequence`
    (:`then_0`
      (`SceneComponent.K2_SetRelativeRotation` (`self.S_Gun`) (`KismetMathLibrary.MakeRotator` (.roll (`SceneComponent.RelativeRotation` (`self.S_Gun`))) (+ (.pitch (`SceneComponent.K2_GetComponentRotation` (`self.CameraBoom`))) (`self.GunPitchScale`)) (.yaw (`SceneComponent.RelativeRotation` (`self.S_Gun`)))) false false))
    (:`then_1`
      (if (`self.bAquiredGun`)
        (bind (_outhit _returnvalue_3) (`KismetSystemLibrary.SphereTraceSingle` :`Start` _returnvalue_2 :`End` (+ _returnvalue_2 (* (`SceneComponent.GetForwardVector` _s_gun_2) (`self.GunTraceRange`))) :`Radius` 20.0 :`TraceChannel` "TraceTypeQuery5" :`DrawDebugType` "ForOneFrame"))
        (if _returnvalue_3
          (bind (_bblockinghit _binitialoverlap _time _distance _location _impactpoint _normal _impactnormal _physmat _hitactor) (`GameplayStatics.BreakHitResult` _outhit))
          (if (`KismetSystemLibrary.DoesImplementInterface` _hitactor "/Game/FurnitureWars/Core/Interfaces/BPI_Furniture.BPI_Furniture_C")
            (set `self.ScalableActor` _hitactor)
            (set `self.bGrabbableObjectFound` true)
            (else
              (set `self.bGrabbableObjectFound` false :!label _label_2)
              (set `self.ScalableActor` null)))
          (else
            (goto _label_2)))))
    (:`then_2`
      (if (`self.bGrabbableObjectFound`)
        (bind _mainhud (message `/Game/FurnitureWars/Core/Interfaces/BPI_GameMode.GetPlayerHUD` _returnvalue))
        (message `/Game/FurnitureWars/Core/Interfaces/BPI_MainHUD.PromptGrab` _mainhud)
        (else
          (bind _mainhud_2 (message `/Game/FurnitureWars/Core/Interfaces/BPI_GameMode.GetPlayerHUD` _returnvalue))
          (message `/Game/FurnitureWars/Core/Interfaces/BPI_MainHUD.RemoveGrab` _mainhud_2))))
    (:`then_3`
      (if (`self.bCurrentlyHolding`)
        (`self.ScaleObject`)))
    (:`then_4`
      (`PhysicsHandleComponent.SetTargetLocation` (`self.PhysicsHandle`) (+ (`SceneComponent.K2_GetComponentLocation` _s_gun) (* (`SceneComponent.GetForwardVector` _s_gun) (`self.GrabbedObjectDistance`)))))
    (:`then_5`)
    (:`then_6`
      (bind _mainhud_3 (message `/Game/FurnitureWars/Core/Interfaces/BPI_GameMode.GetPlayerHUD` (`GameplayStatics.GetGameMode`)))
      (message `/Game/FurnitureWars/Core/Interfaces/BPI_MainHUD.UpdateAreaState` _mainhud_3)
      (message `/Game/FurnitureWars/Core/Interfaces/BPI_MainHUD.UpdateScaleEnergyPercentage` _mainhud_3 (/ (`self.CurrentScaleEnergy`) (`self.MaxScaleEnergy`))))))

(fn `DecideAreaState`
  (returns (CurrentArea :type "/Game/FurnitureWars/Core/Systems/Areas/E_Areas Enum"))
  (bind _bhamputags (`self.BhampuTags`))
  (if (`BlueprintGameplayTagLibrary.HasTag` _bhamputags (struct :`TagName` "Area.Neutral") true)
    (return "NewEnumerator0")
    (elif (`BlueprintGameplayTagLibrary.HasTag` _bhamputags (struct :`TagName` "Area.Hostile"))
      (return "NewEnumerator1")
      (else
        (`KismetSystemLibrary.PrintString` "InvalidArea" true true (struct :`R` 1.0 :`G` 0.046545 :`A` 1.0) 1.0)))))

(fn `GetBhampuTagsContainer`
  (returns (BhampuTags :type "GameplayTagContainer Structure"))
  (return (`self.BhampuTags`)))

(fn `GetCurrentLevel`
  (returns (CurrentLevel :type "/Game/FurnitureWars/Core/Systems/LevelSys/E_LevelNames Enum"))
  (return (`self.CurrentLevel`)))

(fn `GetCurrentStealthState`
  (returns (CurrentStealthState :type "/Game/FurnitureWars/Core/Systems/Stealth/E_StealthStates Enum"))
  (return (`self.CurrentStealthState`)))

(fn `GetWarpLocation`
  (returns (WarpLocation :type "Vector Structure"))
  (return (0.0 0.0 0.0)))

(fn `GrabObject`
  (set `self.CurrentHeldActor` (`self.ScalableActor`))
  (set `self.GrabbedObjectDistance` (`KismetMathLibrary.VSize` (- (`self.K2_GetActorLocation` (`self.CurrentHeldActor`)) (`SceneComponent.K2_GetComponentLocation` (`self.S_Gun`)))))
  (set `self.bCurrentlyHolding` true)
  (bind _mainhud (message `/Game/FurnitureWars/Core/Interfaces/BPI_GameMode.GetPlayerHUD` (`GameplayStatics.GetGameMode`)))
  (message `/Game/FurnitureWars/Core/Interfaces/BPI_MainHUD.PromptScale` _mainhud)
  (bind _staticmeshcomp (message `/Game/FurnitureWars/Core/Interfaces/BPI_Furniture.GetStaticMeshComp` (`self.CurrentHeldActor`)))
  (`PhysicsHandleComponent.GrabComponentAtLocation` (`self.PhysicsHandle`) _staticmeshcomp "None" (`SceneComponent.K2_GetComponentLocation` _staticmeshcomp)))

(fn `ReleaseObject`
  (set `self.CurrentHeldActor` null)
  (set `self.GrabbedObjectDistance` 0.0)
  (set `self.bCurrentlyHolding` false)
  (bind _mainhud (message `/Game/FurnitureWars/Core/Interfaces/BPI_GameMode.GetPlayerHUD` (`GameplayStatics.GetGameMode`)))
  (message `/Game/FurnitureWars/Core/Interfaces/BPI_MainHUD.RemoveScale` _mainhud)
  (`PhysicsHandleComponent.ReleaseComponent` (`self.PhysicsHandle`)))

(fn `ScaleObject`
  (locals (PreviousScaleCache :type "Float (double-precision)"))
  (bind _currentheldactor (`self.CurrentHeldActor`))
  (bind _currentheldactor_2 (`self.CurrentHeldActor`))
  (bind _currentheldactor_3 (`self.CurrentHeldActor`))
  (bind _currentheldactor_4 (`self.CurrentHeldActor`))
  (bind _returnvalue (`KismetMathLibrary.VSize` (`self.GetActorScale3D` _currentheldactor_4)))
  (bind _returnvalue_2 (`KismetMathLibrary.VSize` (`self.GetActorScale3D` _currentheldactor_3)))
  (if (`self.bCanScaleUp`)
    (`/Engine/EditorBlueprintResources/StandardMacros.IsValid` _currentheldactor_4
      (:`Is Valid`
        (bind _maxscale (message `/Game/FurnitureWars/Core/Interfaces/BPI_Furniture.GetMaxScale` _currentheldactor_4))
        (if (< _returnvalue _maxscale)
          (if (< (`self.CurrentScaleEnergy`) (`self.MaxScaleEnergy`))
            (set `local.PreviousScaleCache` _returnvalue)
            (bind _minscale (message `/Game/FurnitureWars/Core/Interfaces/BPI_Furniture.GetMinScale` _currentheldactor))
            (bind _maxscale_2 (message `/Game/FurnitureWars/Core/Interfaces/BPI_Furniture.GetMaxScale` _currentheldactor))
            (`self.SetActorScale3D` (`self.CurrentHeldActor`) (`KismetMathLibrary.MakeVector` (`KismetMathLibrary.FClamp` (.x (* (`self.GetActorScale3D` _currentheldactor) (`self.ScaleUpModifier`))) _minscale _maxscale_2) (`KismetMathLibrary.FClamp` (.y (* (`self.GetActorScale3D` _currentheldactor) (`self.ScaleUpModifier`))) _minscale _maxscale_2) (`KismetMathLibrary.FClamp` (.z (* (`self.GetActorScale3D` _currentheldactor) (`self.ScaleUpModifier`))) _minscale _maxscale_2)))
            (set `self.CurrentScaleEnergy` (`KismetMathLibrary.FClamp` (+ (`self.CurrentScaleEnergy`) (* (- (`KismetMathLibrary.VSize` (`self.GetActorScale3D` (`self.CurrentHeldActor`))) (`local.PreviousScaleCache`)) (`self.UpMultiplier`))) 0.0 (`self.MaxScaleEnergy`)))))))
    (elif (`self.bCanScaleDown`)
      (`/Engine/EditorBlueprintResources/StandardMacros.IsValid` _currentheldactor_3
        (:`Is Valid`
          (bind _minscale_2 (message `/Game/FurnitureWars/Core/Interfaces/BPI_Furniture.GetMinScale` _currentheldactor_3))
          (if (> _returnvalue_2 _minscale_2)
            (if (> (`self.CurrentScaleEnergy`) 0.0)
              (set `local.PreviousScaleCache` _returnvalue_2)
              (bind _minscale_3 (message `/Game/FurnitureWars/Core/Interfaces/BPI_Furniture.GetMinScale` _currentheldactor_2))
              (bind _maxscale_3 (message `/Game/FurnitureWars/Core/Interfaces/BPI_Furniture.GetMaxScale` _currentheldactor_2))
              (`self.SetActorScale3D` (`self.CurrentHeldActor`) (`KismetMathLibrary.MakeVector` (`KismetMathLibrary.FClamp` (.x (* (`self.GetActorScale3D` _currentheldactor_2) (`self.ScaleDownModifier`))) _minscale_3 _maxscale_3) (`KismetMathLibrary.FClamp` (.y (* (`self.GetActorScale3D` _currentheldactor_2) (`self.ScaleDownModifier`))) _minscale_3 _maxscale_3) (`KismetMathLibrary.FClamp` (.z (* (`self.GetActorScale3D` _currentheldactor_2) (`self.ScaleDownModifier`))) _minscale_3 _maxscale_3)))
              (set `self.CurrentScaleEnergy` (`KismetMathLibrary.FClamp` (- (`self.CurrentScaleEnergy`) (* (- (`local.PreviousScaleCache`) (`KismetMathLibrary.VSize` (`self.GetActorScale3D` (`self.CurrentHeldActor`)))) (`self.DownMultiplier`))) 0.0 (`self.MaxScaleEnergy`))))))))))

(fn `UserConstructionScript`)