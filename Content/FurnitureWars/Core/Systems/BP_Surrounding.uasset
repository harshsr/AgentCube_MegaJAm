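; BP_Surrounding is a surrounding scenery actor whose Cube moves vertically in a repeating wave motion.
; BeginPlay caches the Cube's world location, then a looping timer restarts the MoveWave timeline, with both timer interval and play rate scaled by MoveSpeed.
; Each update teleports the Cube to a Z offset from the timeline's Alpha.
; The construction script applies InitialZPosition as a starting height offset.
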(event `self.ReceiveBeginPlay`
  (set `self.InitialLocationcache` (`SceneComponent.K2_GetComponentLocation` (`self.Cube`)))
  (`self.WaveMove`)
  (`KismetSystemLibrary.K2_SetTimerDelegate` (delegate `WaveMove`) (/ 15.0 (`self.MoveSpeed`)) true))

(event `WaveMove`
  (`TimelineComponent.SetPlayRate` (`self.MoveWave`) (`self.MoveSpeed`))
  (bind (_direction _alpha) (`Timeline|MoveWave` :!via `PlayFromStart`)
    (:`Update`
      (`SceneComponent.K2_SetWorldLocation` (`self.Cube`) (`KismetMathLibrary.MakeVector` (.x (`self.InitialLocationcache`)) (.y (`self.InitialLocationcache`)) (+ (.z (`self.InitialLocationcache`)) (* _alpha 100.0))) false true))))

(fn `UserConstructionScript`
  (bind _cube (`self.Cube`))
  (`SceneComponent.K2_SetWorldLocation` _cube (`KismetMathLibrary.MakeVector` (.x (`SceneComponent.K2_GetComponentLocation` _cube)) (.y (`SceneComponent.K2_GetComponentLocation` _cube)) (+ (.z (`SceneComponent.K2_GetComponentLocation` _cube)) (`self.InitialZPosition`))) false false))