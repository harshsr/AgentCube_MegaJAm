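; BP_Elevator is an interactable elevator that rises a fixed height above its starting position, then returns on its own.
; BeginPlay caches the start and target locations, and Interact starts a trip unless one is already running.
; The Elevate timeline drives the ascent, then after a short pause ComeDown drives the descent and snaps to the start.
; Both lerp from the current location each update, so motion compounds rather than directly following the curve.
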(event `self.ReceiveBeginPlay`
  (bind _output_get (set `self.InitialLocation` (`SceneComponent.K2_GetComponentLocation` (`self.Elevator`))))
  (set `self.TargetLocation` (`KismetMathLibrary.MakeVector` (.x _output_get) (.y _output_get) (+ (.z _output_get) 900.0))))

(event `self.Interact`
  (bind _elevator (`self.Elevator`))
  (bind _elevator_2 (`self.Elevator`))
  (if (not (`self.bMoving`))
    (set `self.bMoving` true)
    (bind (_direction _elevation) (`Timeline|Elevate` :!via `PlayFromStart`)
      (:`Update`
        (`SceneComponent.K2_SetWorldLocation` _elevator (`KismetMathLibrary.VLerp` (`SceneComponent.K2_GetComponentLocation` _elevator) (`self.TargetLocation`) _elevation) false true))
      (:`Finished`
        (`KismetSystemLibrary.Delay` 1.0)
        (bind (_direction_2 _elevation_2) (`Timeline|ComeDown` :!via `PlayFromStart`)
          (:`Update`
            (`SceneComponent.K2_SetWorldLocation` _elevator_2 (`KismetMathLibrary.VLerp` (`SceneComponent.K2_GetComponentLocation` _elevator_2) (`self.InitialLocation`) _elevation_2) false true))
          (:`Finished`
            (`SceneComponent.K2_SetWorldLocation` (`self.Elevator`) (`self.InitialLocation`) false true)
            (set `self.bMoving` false)))))))

(fn `UserConstructionScript`)