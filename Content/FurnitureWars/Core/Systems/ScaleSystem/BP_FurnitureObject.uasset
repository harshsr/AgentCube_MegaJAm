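; Destructible physics furniture for Furniture Wars, optionally flagged as a level objective, exposing its mesh and min/max scale through getters.
; Non-Ground hits subtract health by both components' velocities, updating a health widget that turns toward the player camera each tick.
; Below zero health it fires a radial impulse, then explodes or, as an objective, fails the level, before destruction.
; Objective pieces update BP_ObjectivePlace counts and the HUD on overlap.
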(event `self.ReceiveTick`
  (params (DeltaSeconds :type "Float (single-precision)"))
  (bind _widget (`self.Widget`))
  (`SceneComponent.K2_SetWorldRotation` _widget (`KismetMathLibrary.FindLookAtRotation` (`SceneComponent.K2_GetComponentLocation` _widget) (`SceneComponent.K2_GetComponentLocation` (`Bhampu.MainCamera` (cast `/Game/FurnitureWars/Core/Bhampu/BP_Bhampu` (`GameplayStatics.GetPlayerPawn` 0) :!pure true)))) false true))

(event `self.ReceiveBeginPlay`
  (bind _maxhealth (`self.MaxHealth`))
  (bind _output_get (set `self.Health` _maxhealth))
  (message `/Game/FurnitureWars/Core/Interfaces/BPI_Furniture.UpdateHealthPercentage` (`WidgetComponent.GetUserWidgetObject` (`self.Widget`)) (/ _output_get _maxhealth)))

(event `self.StaticMeshComponent.OnComponentHit`
  (params (HitComponent :type "PrimitiveComponent Object Reference") (OtherActor :type "Actor Object Reference") (OtherComp :type "PrimitiveComponent Object Reference") (NormalImpulse :type "Vector Structure") (Hit :type "HitResult Structure (by ref)"))
  (if (not (`self.ActorHasTag` OtherActor "Ground"))
    (bind _returnvalue (`PrimitiveComponent.GetPhysicsLinearVelocity` OtherComp "None"))
    (bind _returnvalue_2 (`PrimitiveComponent.GetPhysicsLinearVelocity` HitComponent "None"))
    (bind _output_get (set `self.Health` (- (`self.Health`) (+ (* (`KismetMathLibrary.VSize` _returnvalue_2) (`self.DamageModifier`)) (* (`KismetMathLibrary.VSize` _returnvalue) (`self.DamageModifier`))))))
    (message `/Game/FurnitureWars/Core/Interfaces/BPI_Furniture.UpdateHealthPercentage` (`WidgetComponent.GetUserWidgetObject` (`self.Widget`)) (/ _output_get (`self.MaxHealth`)))
    (if (< (`self.Health`) 0.0)
      (`RadialForceComponent.FireImpulse` (`self.RadialForce`))
      (if (`self.bObjective`)
        (message `/Game/FurnitureWars/Core/Interfaces/BPI_Tutorial.SuccessInLevel` (`GameplayStatics.GetGameMode`) false "NewEnumerator1")
        (else
          (`GameplayStatics.SpawnEmitterAtLocation` "/Game/M5VFXVOL2/Particles/Explosion/Fire_Exp_03.Fire_Exp_03" (`self.K2_GetActorLocation`))
          (`GameplayStatics.SpawnSound2D` "/Game/FurnitureWars/Art/AudioLib/A_BitExplosion.A_BitExplosion" 1.0 1.0 0.0 null)))
      (`KismetSystemLibrary.Delay` 0.05)
      (`self.K2_DestroyActor`))))

(event `self.StaticMeshComponent.OnComponentBeginOverlap`
  (params (OverlappedComponent :type "PrimitiveComponent Object Reference") (OtherActor :type "Actor Object Reference") (OtherComp :type "PrimitiveComponent Object Reference") (OtherBodyIndex :type Integer) (bFromSweep :type Boolean) (SweepResult :type "HitResult Structure (by ref)"))
  (bind _asbp_objective_place (cast `/Game/FurnitureWars/Core/Systems/ScaleSystem/BP_ObjectivePlace` OtherActor))
  (if (`self.bObjective`)
    (set `/Game/FurnitureWars/Core/Systems/ScaleSystem/BP_ObjectivePlace.CurrentObjectives` (+ (`/Game/FurnitureWars/Core/Systems/ScaleSystem/BP_ObjectivePlace.CurrentObjectives` _asbp_objective_place) 1) _asbp_objective_place)
    (bind _mainhud (message `/Game/FurnitureWars/Core/Interfaces/BPI_GameMode.GetPlayerHUD` (`GameplayStatics.GetGameMode`)))
    (message `/Game/FurnitureWars/Core/Interfaces/BPI_MainHUD.AddObjective` _mainhud)))

(event `self.StaticMeshComponent.OnComponentEndOverlap`
  (params (OverlappedComponent :type "PrimitiveComponent Object Reference") (OtherActor :type "Actor Object Reference") (OtherComp :type "PrimitiveComponent Object Reference") (OtherBodyIndex :type Integer))
  (bind _asbp_objective_place (cast `/Game/FurnitureWars/Core/Systems/ScaleSystem/BP_ObjectivePlace` OtherActor))
  (if (`self.bObjective`)
    (set `/Game/FurnitureWars/Core/Systems/ScaleSystem/BP_ObjectivePlace.CurrentObjectives` (+ (`/Game/FurnitureWars/Core/Systems/ScaleSystem/BP_ObjectivePlace.CurrentObjectives` _asbp_objective_place) -1) _asbp_objective_place)
    (bind _mainhud (message `/Game/FurnitureWars/Core/Interfaces/BPI_GameMode.GetPlayerHUD` (`GameplayStatics.GetGameMode`)))
    (message `/Game/FurnitureWars/Core/Interfaces/BPI_MainHUD.RemoveObjective` _mainhud)))

(fn `GetMaxScale`
  (returns (MaxScale :type "Float (double-precision)"))
  (return (`self.MaxScale`)))

(fn `GetMinScale`
  (returns (MinScale :type "Float (double-precision)"))
  (return (`self.MinScale`)))

(fn `GetStaticMeshComp`
  (returns (StaticMeshComp :type "StaticMeshComponent Object Reference"))
  (return (`self.StaticMeshComponent`)))

(fn `UserConstructionScript`)