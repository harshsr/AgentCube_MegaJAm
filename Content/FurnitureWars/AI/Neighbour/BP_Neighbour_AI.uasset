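; Neighbour AI character that patrols points, detects the player and shows dialogue when interacted with.
; Getters expose detection and ask-to-leave state, and serve looping move points, with GetWaitTime also advancing the index.
; Events accumulate or reset a detection timer; spotting the player hiding changes their stealth state and sets the neighbour's walk speed.
; Interact cycles response lines into a character-by-character widget update with its delay disconnected, and FacePlayer interpolates rotation toward the player.
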(event `self.ReceiveTick`
  (params (DeltaSeconds :type "Float (single-precision)"))
  (bind _output_get (set `self.Delta Seconds` DeltaSeconds)))

(event `self.Interact`
  ;[1 1 1] Player Interaction
  (if (>= (`self.Responseindex`) (`KismetArrayLibrary.Array_Length` (`self.ResponseToInteract`)))
    (set `self.Responseindex` 0))
  (`self.DrawDialog` (`|GetArrayItem` (`self.ResponseToInteract`) (`self.Responseindex`)))
  (`/Engine/EditorBlueprintResources/StandardMacros.IncrementInt` (`self.Responseindex`)))

(event `self.AdvanceDetectionTime`
  (set `self.CurrentDetectionTime` (+ (`self.CurrentDetectionTime`) (`self.Delta Seconds`))))

(event `self.ResetCurrentDetectionTime`
  (set `self.CurrentDetectionTime` 0.0)
  (set `self.bSpottedHiding` false))

(event `self.CheckSpottedHiding`
  (if (`self.bSeeingCustom`)
    (message `/Game/FurnitureWars/Core/Interfaces/BPI_StealthSystem.ModifyCurrentStealthState` (`GameplayStatics.GetPlayerPawn` 0) "NewEnumerator2")
    (set `self.bSpottedHiding` true)
    (set `CharacterMovementComponent.MaxWalkSpeed` 450.0 (`self.CharacterMovement`))))

(event `self.DrawDialog`
  (params (DialogString :type String))
  (set `self.DialogString` "")
  (for _array_element (`KismetStringLibrary.GetCharacterArrayFromString` DialogString)
    (bind _output_get (set `self.DialogString` (`KismetStringLibrary.Concat_StrStr` (`self.DialogString`) _array_element)))
    (message `/Game/FurnitureWars/AI/Neighbour/BPI_Neighbour.UpdateDialougeOnUI` (`WidgetComponent.GetUserWidgetObject` (`self.DialogWidget`)) (`KismetTextLibrary.Conv_StringToText` _output_get)))
  (message `/Game/FurnitureWars/AI/Neighbour/BPI_Neighbour.UpdateDialougeOnUI` (`WidgetComponent.GetUserWidgetObject` (`self.DialogWidget`)) (`KismetTextLibrary.Conv_StringToText` (`self.DialogString`))))

(event `self.FacePlayer`
  (`self.K2_SetActorRotation` (`KismetMathLibrary.RInterpTo` (`self.K2_GetActorRotation`) (`KismetMathLibrary.FindLookAtRotation` (`self.K2_GetActorLocation`) (`self.K2_GetActorLocation` (`GameplayStatics.GetPlayerPawn` 0))) 1.0 5.0)))

(fn `GetAskToLeave`
  (returns (AskToLeave :type String))
  (return (`self.AskToLeave`)))

(fn `GetCurrentDetectionTime`
  (returns (CurrentDetectionTime :type "Float (double-precision)"))
  (return (`self.CurrentDetectionTime`)))

(fn `GetDesiredDetectionTime`
  (returns (DesiredDetectionTime :type "Float (double-precision)"))
  (return (`self.DesiredDetectionTime`)))

(fn `GetNextMovePoint`
  (returns (MovePoint :type "Actor Object Reference"))
  (return (`|GetArrayItem` (`self.MovePoints`) (`self.MovePointIndex`))))

(fn `GetSeeingJonna`
  (returns (bSeeingJonna :type Boolean))
  (return (`self.bSeeingCustom`)))

(fn `GetSpottedHiding`
  (returns (bSpottedHiding :type Boolean))
  (return (`self.bSpottedHiding`)))

(fn `GetWaitTime`
  (returns (WaitTime :type "Float (double-precision)"))
  (locals (WaitTimeCache :type "Float (double-precision)"))
  (set `local.WaitTimeCache` (`|GetArrayItem` (`self.WaitTime`) (`self.MovePointIndex`)))
  (bind _output_get (set `self.MovePointIndex` (+ (`self.MovePointIndex`) 1)))
  (if (== _output_get (`KismetArrayLibrary.Array_Length` (`self.MovePoints`)))
    (set `self.MovePointIndex` 0))
  (return (`local.WaitTimeCache`)))

(fn `UserConstructionScript`)